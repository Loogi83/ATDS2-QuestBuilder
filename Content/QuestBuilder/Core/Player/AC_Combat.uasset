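; Player combat component that performs a forward area attack for its owning actor.
; Attack runs a multi-sphere object trace from the owner along its forward vector, using configurable length and radius, filtered to one object type and ignoring the owner.
; Every hit receives base damage through ApplyDamage, and the trace draws timed debug shapes.
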(event Custom|Attack
  (bind _returnvalue (Components|GetOwner))
  (bind _returnvalue_2 (Transformation|GetActorLocation _returnvalue))
  (bind _outhits (Collision|MultiSphereTraceForObjects _returnvalue_2 (+ _returnvalue_2 (* (Transformation|GetActorForwardVector _returnvalue) (Variables|Default|GetTraceLength))) (Variables|Default|GetTraceRadius) (Utilities|Array|MakeArray "ObjectTypeQuery7") false (Utilities|Array|MakeArray (Components|GetOwner)) "ForDuration"))
  (for _array_element _outhits
    (Game|Damage|ApplyDamage (.HitActor (Collision|BreakHitResult _array_element)) (Variables|Default|GetBase%20Damage) 0 0)))