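; AC_Health is a player health component that tracks damage, regenerates health and signals death.
; Init binds the owner's damage event, fills health and creates the WBP_Health widget, which updates as health changes.
; Non-lethal damage restarts a five-second retriggerable delay before a looping timer restores one point per tick until health exactly equals the maximum.
; Lethal damage calls the EDeath dispatcher.
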(event Custom|Init
  (params (Owner :type BP%20Third%20Person%20Character%20Object%20Reference))
  ;[1 1 1] Init
  (EventDispatchers|BindEventtoOnTakeAnyDamage Owner (EventDispatchers|CreateEvent :!event Custom|TakeAnyDamage))
  (Variables|Default|SetCurrentHealth (Variables|Default|GetMaxHealth))
  (bind _returnvalue (UserInterface|CreateWidget "/Game/QuestBuilder/Core/UI/WBP_Health.WBP_Health_C"))
  (bind _output_get (Variables|Default|SetHealthUI _returnvalue))
  (Default|Init _output_get self)
  (UserInterface|Viewport|AddtoViewport _output_get 0))

(event Custom|TakeAnyDamage
  (params (DamagedActor :type Actor%20Object%20Reference) (Damage :type Float%20%28single-precision%29) (DamageType :type Damage%20Type%20Object%20Reference) (InstigatedBy :type Controller%20Object%20Reference) (DamageCauser :type Actor%20Object%20Reference))
  ;[1 1 1] Take Damage 😫
  (if (> (- (Variables|Default|GetCurrentHealth) Damage) 0.0)
    (bind _output_get (Variables|Default|SetCurrentHealth (- (Variables|Default|GetCurrentHealth) Damage)))
    (Default|UpdateHealth (Variables|Default|GetHealthUI) _output_get)
    (Utilities|FlowControl|RetriggerableDelay 5.0)
    (CallFunction|RegenHealth)
    (else
      (Default|CallEDeath))))

(event Custom|RegenHealth
  ;[1 1 1] Regen Health
  (bind _returnvalue (Utilities|Time|SetTimerbyEvent (delegate Custom|Restore) (Variables|Default|GetRegenSpeed) true))
  (Variables|Default|SetRegenHandle _returnvalue))

(event Custom|Restore
  ;[1 1 1] Regen Health
  (bind _output_get (Variables|Default|SetCurrentHealth (+ (Variables|Default|GetCurrentHealth) 1.0)))
  (Default|UpdateHealth (Variables|Default|GetHealthUI) _output_get)
  (if (== _output_get (Variables|Default|GetMaxHealth))
    (Utilities|Time|ClearandInvalidateTimerbyHandle (Variables|Default|GetRegenHandle))))