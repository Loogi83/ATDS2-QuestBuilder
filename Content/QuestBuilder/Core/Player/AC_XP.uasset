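; AC_XP is a player component that tracks XP and level and shows them in a WBP_XP widget.
; Init creates the widget, passes itself to it and adds it to the viewport.
; RewardXP adds XP; on reaching the target it levels up, carries over the surplus, scales the target by a rounded multiplier and updates the widget.
; It then calls itself with zero XP, so one reward can grant several levels.
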(event Custom|Init
  (params (Owner :type BP%20Third%20Person%20Character%20Object%20Reference))
  (bind _returnvalue (UserInterface|CreateWidget "/Game/QuestBuilder/Core/UI/WBP_XP.WBP_XP_C"))
  (bind _output_get (Variables|Default|SetUI _returnvalue))
  (Default|Init _output_get self)
  (UserInterface|Viewport|AddtoViewport _output_get 0))

(fn RewardXP
  (params (XP%20to%20Reward :type Float%20%28double-precision%29))
  (bind _ui (Variables|Default|GetUI))
  (bind _output_get (Variables|Default|SetXP (+ XP%20to%20Reward (Variables|Default|GetXP))))
  (if (< _output_get (Variables|Default|GetTargetXP))
    (Default|UpdateXP (Variables|Default|GetUI) (Variables|Default|GetXP))
    (else
      (Math|Integer|IncrementInt (Variables|Default|GetLevel)
        (:%20%20
          (Variables|Default|SetXP (- _output_get (Variables|Default|GetTargetXP)))
          (Variables|Default|SetTargetXP (Math|Conversions|ToFloat(Integer) (Math|Float|Round (* (Variables|Default|GetTargetXP) (Variables|Default|GetTargetMultiplier)))))
          (Default|UpdateLevel _ui (Variables|Default|GetLevel))
          (Default|UpdateXP _ui (Variables|Default|GetXP))
          (CallFunction|RewardXP 0.0))))))