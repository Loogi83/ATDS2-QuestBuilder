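; AC_XP is an experience component that tracks XP toward a target and displays it through a WBP_XP widget.
; Init creates the widget, passes itself to it and adds it to the viewport.
; RewardXP adds the reward to XP and updates the widget while below TargetXP.
; On reaching the target it subtracts TargetXP once to carry the remainder, without refreshing the widget.
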(event Custom|Init
  (params (Owner :type BP%20Third%20Person%20Character%20Object%20Reference))
  (bind _returnvalue (UserInterface|CreateWidget "/Game/QuestBuilder/Core/WBP_XP.WBP_XP_C"))
  (bind _output_get (Variables|Default|SetUI _returnvalue))
  (Default|Init _output_get self)
  (UserInterface|Viewport|AddtoViewport _output_get 0))

(fn RewardXP
  (params (XP%20to%20Reward :type Float%20%28double-precision%29))
  (bind _targetxp (Variables|Default|GetTargetXP))
  (bind _output_get (Variables|Default|SetXP (+ XP%20to%20Reward (Variables|Default|GetXP))))
  (if (< _output_get _targetxp)
    (Default|UpdateXP (Variables|Default|GetUI) (Variables|Default|GetXP))
    (else
      (Variables|Default|SetXP (- _output_get _targetxp)))))