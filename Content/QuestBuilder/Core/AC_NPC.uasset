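; Actor component from the Quest Builder core that gives an NPC an interaction range tied to its quest data.
; Init adds a visible sphere collider to the owner, sized by InteractRadius, and binds its overlap events at runtime.
; When the player character enters, it prints the quest type and marker location; on exit, it prints the XP reward.
; The overlaps only print this debug text.
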(event Custom|Init
  (bind _returnvalue (Game|AddComponentbyClass (Components|GetOwner) "/Script/Engine.SphereComponent" false))
  (bind _output_get (Variables|Default|SetCollider _returnvalue))
  (Components|Sphere|SetSphereRadius _output_get (Variables|Default|GetInteractRadius) true)
  (Collision|BindEventtoOnComponentBeginOverlap (Variables|Default|GetCollider) (EventDispatchers|CreateEvent :!event Custom|BeginOverlap))
  (Collision|BindEventtoOnComponentEndOverlap (Variables|Default|GetCollider) (EventDispatchers|CreateEvent :!event Custom|EndOverlap))
  (Development|SetHiddeninGame (Variables|Default|GetCollider) false false))

(event Custom|BeginOverlap
  (params (OverlappedComponent :type Primitive%20Component%20Object%20Reference) (OtherActor :type Actor%20Object%20Reference) (OtherComp :type Primitive%20Component%20Object%20Reference) (OtherBodyIndex :type Integer) (bFromSweep :type Boolean) (SweepResult :type Hit%20Result%20Structure%20%28by%20ref%29))
  (bind _questdata (Variables|Default|GetQuestData))
  (if (== OtherActor (Game|GetPlayerCharacter 0))
    (Development|PrintString (Utilities|String|Append "Quest Type: " (Utilities|String|EnumtoString (Variables|/Game/QuestBuilder/Core/QuestData/PDA_QuestDataParent.PDA_QuestDataParent_C|GetQuestType _questdata)) " Location: " (Utilities|String|ToString(Vector) (Variables|/Game/QuestBuilder/Core/QuestData/PDA_QuestDataParent.PDA_QuestDataParent_C|GetMarkerLocation _questdata))))))

(event Custom|EndOverlap
  (params (OverlappedComponent :type Primitive%20Component%20Object%20Reference) (OtherActor :type Actor%20Object%20Reference) (OtherComp :type Primitive%20Component%20Object%20Reference) (OtherBodyIndex :type Integer))
  (if (== OtherActor (Game|GetPlayerCharacter 0))
    (Development|PrintString (Utilities|String|Append "Reward: " (Utilities|String|ToString(Float) (Variables|/Game/QuestBuilder/Core/QuestData/PDA_QuestDataParent.PDA_QuestDataParent_C|GetRewardXP (Variables|Default|GetQuestData)))))))