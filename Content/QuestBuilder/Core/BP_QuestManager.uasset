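; Quest manager Blueprint that starts a location-based objective from its quest data when Init is called.
; StartQuest spawns a BP_QuestMarker at the target, binds to its location-reached dispatcher and passes the marker position to the compass component.
; It flags the quest active and creates the objective widget if none exists.
; ObjectiveReached currently only prints a completion message.
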(event Custom|ObjectiveReached
  (Development|PrintString "Objective Complete"))

(event Custom|Init
  (CallFunction|StartQuest (Variables|/Game/QuestBuilder/Core/QuestData/PDA_QuestDataParent.PDA_QuestDataParent_C|GetMarkerLocation (Variables|Default|GetQuestData))))

(fn ConstructionScript)

(fn StartQuest
  (params (Spawn%20Transform%20Location :type Vector))
  (bind _ac_compass (Variables|Default|GetAC%20Compass))
  (bind _returnvalue (Game|SpawnActorfromClass "/Game/QuestBuilder/Core/BP_QuestMarker.BP_QuestMarker_C" (Math|Transform|MakeTransform Spawn%20Transform%20Location "0, 0, 0" "1.000000,1.000000,1.000000") "Undefined" 0 0))
  (bind _output_get (Variables|Default|SetQuestMarker _returnvalue))
  (EventDispatchers|BindEventtoEDLocationReached _output_get (EventDispatchers|CreateEvent :!event Custom|ObjectiveReached))
  (Variables|/Game/QuestBuilder/Core/Compass/AC_Compass.AC_Compass_C|SetObjectiveLocation _ac_compass (Transformation|GetActorLocation (Variables|Default|GetQuestMarker)))
  (Default|SetObjective (Variables|/Game/QuestBuilder/Core/Compass/AC_Compass.AC_Compass_C|GetCompassRef _ac_compass))
  (Variables|Default|SetbQuestActive? true)
  (Variables|Default|GetObjectiveUI
    (:then)
    (:else
      (bind _returnvalue_2 (UserInterface|CreateWidget "/Game/QuestBuilder/Core/UI/WBP_Objective.WBP_Objective_C"))
      (bind _output_get_2 (Variables|Default|SetObjectiveUI _returnvalue_2))
      (UserInterface|Viewport|AddtoViewport _output_get_2 0))))