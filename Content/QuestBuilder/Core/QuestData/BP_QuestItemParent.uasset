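; BP_QuestItemParent is a base actor for collectible quest items that the player picks up by walking into them.
; On init, a Hover timeline bobs the static mesh up and down along its local Z axis.
; When the player character overlaps the sphere, it calls the item-picked-up event dispatcher with itself and then destroys the actor.
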(event OnComponentBeginOverlap(Sphere)
  (params (OverlappedComponent :type Primitive%20Component%20Object%20Reference) (OtherActor :type Actor%20Object%20Reference) (OtherComp :type Primitive%20Component%20Object%20Reference) (OtherBodyIndex :type Integer) (bFromSweep :type Boolean) (SweepResult :type Hit%20Result%20Structure%20%28by%20ref%29))
  ;[1 1 1] Begin Overlap
  (if (== OtherActor (Game|GetPlayerCharacter 0))
    (Default|CallEItemPickedUp self)
    (Actor|DestroyActor)))

(event Custom|Init
  ;[1 1 1] Hover
  (bind _alpha (Timeline|Hover PlayFromStart)
    (:Update
      (Transformation|SetRelativeLocation (Variables|Default|GetStaticMesh) (Math|Vector|Lerp(Vector) "0.000000,0.000000,10.000000" "0.000000,0.000000,-10.000000" _alpha) false false))))

(fn ConstructionScript)