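; Quest manager that runs one active Fetch, Reach or Kill quest, from start at an NPC to XP reward.
; StartQuest spawns a location marker, plus an enemy for Kill quests, and updates the objective list and compass.
; Marker-reached and enemy-killed events advance objectives by quest type.
; Reach completes on arrival, while Fetch and Kill use a Return flag to require going back to the NPC first.
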(event Custom|EnemyKilled
  (CallFunction|ClearObjective)
  (CallFunction|ReturntoNPC))

(event Custom|Init
  ;[1 1 1] Init
  (bind _asbp_third_person_character (Utilities|Casting|CastToBP_ThirdPersonCharacter (Game|GetPlayerCharacter 0)))
  (Variables|Default|SetAC%20XP (Variables|/Game/ThirdPerson/Blueprints/BP_ThirdPersonCharacter.BP_ThirdPersonCharacter_C|GetAC_XP _asbp_third_person_character))
  (Variables|Default|SetAC%20Compass (Variables|/Game/ThirdPerson/Blueprints/BP_ThirdPersonCharacter.BP_ThirdPersonCharacter_C|GetAC_Compass _asbp_third_person_character))
  (bind _returnvalue (UserInterface|CreateWidget "/Game/QuestBuilder/Core/UI/WBP_ObjectiveList.WBP_ObjectiveList_C"))
  (bind _output_get (Variables|Default|SetObjectiveUI _returnvalue))
  (UserInterface|Viewport|AddtoViewport _output_get 0))

(event Custom|ObjectiveReached
  ;[1 1 1] Objective Reached
  (if (Variables|Default|GetReturn?)
    (Variables|Default|SetReturn? false)
    (CallFunction|CompleteQuest :!label _label)
    (else
      (switch Utilities|FlowControl|Switch|SwitchonE_QuestType (Variables|/Game/QuestBuilder/Core/QuestData/PDA_QuestDataParent.PDA_QuestDataParent_C|GetQuestType (Variables|Default|GetQuestData))
        (:NewEnumerator0
          (CallFunction|ClearObjective)
          (CallFunction|ReturntoNPC))
        (:NewEnumerator1
          (goto _label))
        (:NewEnumerator2
          (CallFunction|ClearObjective)
          (bind _objective (Default|AddObjective (Variables|Default|GetObjectiveUI) "Kill Enemy"))
          (Utilities|Array|Add (Variables|Default|GetCurrentObjectiveUI) _objective))))))

(event EventBeginPlay
  ;[1 1 1] Begin Play
  (CallFunction|Init))

(fn ConstructionScript)

(fn StartQuest
  (params (QuestData :type PDA%20Quest%20Data%20Parent%20Object%20Reference) (NPC :type BP%20NPC%20Object%20Reference))
  (Variables|Default|SetNPC NPC)
  (bind _output_get (Variables|Default|SetQuestData QuestData))
  (CallFunction|CreateMarker (Variables|/Game/QuestBuilder/Core/QuestData/PDA_QuestDataParent.PDA_QuestDataParent_C|GetMarkerLocation _output_get))
  (Variables|Default|SetbQuestActive? true)
  (if (Utilities|Enum|NotEqual(Enum) (Variables|/Game/QuestBuilder/Core/QuestData/PDA_QuestDataParent.PDA_QuestDataParent_C|GetQuestType (Variables|Default|GetQuestData)) "NewEnumerator2")
    _
    (else
      (bind _returnvalue (Game|SpawnActorfromClass "/Game/QuestBuilder/Core/Enemy/BP_Enemy.BP_Enemy_C" (Math|Transform|MakeTransform (+ (Variables|/Game/QuestBuilder/Core/QuestData/PDA_QuestDataParent.PDA_QuestDataParent_C|GetMarkerLocation _output_get) "0.000000,0.000000,90.000000")) "AlwaysSpawn" 0 0))
      (Default|Init _returnvalue)
      (EventDispatchers|BindEventtoEEnemyDestroyed (Variables|/Game/QuestBuilder/Core/Enemy/BP_Enemy.BP_Enemy_C|GetAC_Enemy _returnvalue) (EventDispatchers|CreateEvent :!event Custom|EnemyKilled))))
  (bind _objective (Default|AddObjective (Variables|Default|GetObjectiveUI) "Reach Objective Point"))
  (Utilities|Array|Add (Variables|Default|GetCurrentObjectiveUI) _objective))

(fn ReturntoNPC
  (CallFunction|CreateMarker (Transformation|GetActorLocation (Variables|Default|GetNPC)))
  (Variables|Default|SetbQuestActive? true)
  (bind _objective (Default|AddObjective (Variables|Default|GetObjectiveUI) "Return"))
  (Utilities|Array|Add (Variables|Default|GetCurrentObjectiveUI) _objective)
  (Variables|Default|SetReturn? true))

(fn CreateMarker
  (params (SpawnLocation :type Vector))
  (bind _ac_compass (Variables|Default|GetAC%20Compass))
  (bind _returnvalue (Game|SpawnActorfromClass "/Game/QuestBuilder/Core/QuestData/BP_QuestMarker.BP_QuestMarker_C" (Math|Transform|MakeTransform SpawnLocation "0, 0, 0" "1.000000,1.000000,1.000000") "Undefined" 0 0))
  (bind _output_get (Variables|Default|SetQuestMarker _returnvalue))
  (EventDispatchers|BindEventtoEDLocationReached _output_get (EventDispatchers|CreateEvent :!event Custom|ObjectiveReached))
  (Variables|/Game/QuestBuilder/Core/Compass/AC_Compass.AC_Compass_C|SetObjectiveLocation _ac_compass (Transformation|GetActorLocation (Variables|Default|GetQuestMarker)))
  (Default|SetObjective (Variables|/Game/QuestBuilder/Core/Compass/AC_Compass.AC_Compass_C|GetCompassRef _ac_compass)))

(fn CompleteQuest
  (Default|RewardXP (Variables|Default|GetAC%20XP) (Variables|/Game/QuestBuilder/Core/QuestData/PDA_QuestDataParent.PDA_QuestDataParent_C|GetRewardXP (Variables|Default|GetQuestData)))
  (CallFunction|ClearObjective))

(fn ClearObjective
  (bind _currentobjectiveui (Variables|Default|GetCurrentObjectiveUI))
  (bind _output (Utilities|Array|Get(acopy) _currentobjectiveui))
  (Variables|Default|SetbQuestActive? false)
  (Widget|RemovefromParent _output)
  (Utilities|Array|RemoveItem _currentobjectiveui _output)
  (Default|ClearObjective (Variables|/Game/QuestBuilder/Core/Compass/AC_Compass.AC_Compass_C|GetCompassRef (Variables|Default|GetAC%20Compass))))