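; Enemy component that gives its owning actor health, a health widget and death handling.
; Init adds a sphere collider and a screen-space WBP_Enemy widget at runtime, shown only while the player overlaps the sphere.
; Damage taken by the owner updates the widget, or fires the enemy-destroyed dispatcher and destroys the owner when health runs out.
; A separate ApplyDamage event deals base damage to the overlapped actor.
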(event Custom|ApplyDamage
  ;[1 1 1] Begin Overlap
  ;;[1 0.05098 0] Apply Damage
  (Game|Damage|ApplyDamage (stale Custom|BeginOverlap OtherActor) (Variables|Default|GetBase%20Damage) 0 0))

(event Custom|BeginOverlap
  (params (OverlappedComponent :type Primitive%20Component%20Object%20Reference) (OtherActor :type Actor%20Object%20Reference) (OtherComp :type Primitive%20Component%20Object%20Reference) (OtherBodyIndex :type Integer) (bFromSweep :type Boolean) (SweepResult :type Hit%20Result%20Structure%20%28by%20ref%29))
  ;[1 1 1] Begin Overlap
  (if (== OtherActor (Game|GetPlayerCharacter 0))
    (Widget|SetVisibility (Variables|Default|GetWidget) "Visible")))

(event Custom|EndOverlap
  (params (OverlappedComponent :type Primitive%20Component%20Object%20Reference) (OtherActor :type Actor%20Object%20Reference) (OtherComp :type Primitive%20Component%20Object%20Reference) (OtherBodyIndex :type Integer))
  ;[1 1 1] End Overlap
  (if (== OtherActor (Game|GetPlayerCharacter 0))
    (Widget|SetVisibility (Variables|Default|GetWidget) "Hidden")))

(event Custom|Init
  ;[1 1 1] Init
  (bind _output_get (Variables|Default|SetOwner (Components|GetOwner)))
  (CallFunction|AddCollider _output_get)
  (Variables|Default|SetCurrentHealth (Variables|Default|GetMaxHealth))
  (CallFunction|AddHealthUI)
  (EventDispatchers|BindEventtoOnTakeAnyDamage (Components|GetOwner) (EventDispatchers|CreateEvent :!event Custom|TakeAnyDamage)))

(event Custom|TakeAnyDamage
  (params (DamagedActor :type Actor%20Object%20Reference) (Damage :type Float%20%28single-precision%29) (DamageType :type Damage%20Type%20Object%20Reference) (InstigatedBy :type Controller%20Object%20Reference) (DamageCauser :type Actor%20Object%20Reference))
  ;[1 1 1] Take Any Damage
  (if (> (- (Variables|Default|GetCurrentHealth) Damage) 0.0)
    (bind _output_get (Variables|Default|SetCurrentHealth (- (Variables|Default|GetCurrentHealth) Damage)))
    (Default|UpdateUI (Variables|Default|GetWidget) _output_get)
    (else
      ;;[1 0.07208 0] Death 💀
      (Default|CallEEnemyDestroyed)
      (Actor|DestroyActor (Components|GetOwner)))))

(fn AddCollider
  (params (Owner :type Actor%20Object%20Reference))
  (bind _returnvalue (Game|AddComponentbyClass Owner "/Script/Engine.SphereComponent" false))
  (bind _output_get (Variables|Default|SetCollider _returnvalue))
  (Components|Sphere|SetSphereRadius _output_get (Variables|Default|GetInteractRadius) true)
  (Collision|BindEventtoOnComponentBeginOverlap (Variables|Default|GetCollider) (EventDispatchers|CreateEvent :!event Custom|BeginOverlap))
  (Collision|BindEventtoOnComponentEndOverlap (Variables|Default|GetCollider) (EventDispatchers|CreateEvent :!event Custom|EndOverlap)))

(fn AddHealthUI
  (bind _returnvalue (Game|AddComponentbyClass (Variables|Default|GetOwner) "/Script/UMG.WidgetComponent" false (Math|Transform|MakeTransform "0.000000,0.000000,100.000000")))
  (bind _returnvalue_2 (UserInterface|CreateWidget "/Game/QuestBuilder/Core/NPC/WBP_Enemy.WBP_Enemy_C"))
  (Default|Init _returnvalue_2 self)
  (Variables|Default|SetWidget _returnvalue_2)
  (UserInterface|SetWidget _returnvalue _returnvalue_2)
  (Class|WidgetComponent|SetWidgetSpace _returnvalue "Screen")
  (Widget|SetVisibility (Variables|Default|GetWidget) "Hidden"))