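; Actor component that turns its owning NPC into a quest giver in the QuestBuilder system.
; On Init it adds a hidden screen-space prompt widget and a sphere collider that shows it while the player overlaps, and finds the BP_QuestManager.
; Interacting offers the quest, completes it on return, or opens a state-dependent text box.
; Dialogue widgets take UI-only input and disable player movement.
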(event Custom|Init
  (bind _returnvalue (Components|GetOwner))
  ;[1 1 1] Init
  (CallFunction|AddInteractWidget _returnvalue)
  (CallFunction|AddCollider _returnvalue)
  (bind _returnvalue_2 (Actor|GetActorOfClass "/Game/QuestBuilder/Core/QuestData/BP_QuestManager.BP_QuestManager_C"))
  (Variables|Default|SetManager _returnvalue_2))

(event Custom|BeginOverlap
  (params (OverlappedComponent :type Primitive%20Component%20Object%20Reference) (OtherActor :type Actor%20Object%20Reference) (OtherComp :type Primitive%20Component%20Object%20Reference) (OtherBodyIndex :type Integer) (bFromSweep :type Boolean) (SweepResult :type Hit%20Result%20Structure%20%28by%20ref%29))
  ;[1 1 1] Begin Overlap
  (if (== OtherActor (Game|GetPlayerCharacter 0))
    (Rendering|SetVisibility (Variables|Default|GetWidget) true false)))

(event Custom|EndOverlap
  (params (OverlappedComponent :type Primitive%20Component%20Object%20Reference) (OtherActor :type Actor%20Object%20Reference) (OtherComp :type Primitive%20Component%20Object%20Reference) (OtherBodyIndex :type Integer))
  ;[1 1 1] End Overlap
  (if (== OtherActor (Game|GetPlayerCharacter 0))
    (Rendering|SetVisibility (Variables|Default|GetWidget) false false)))

(event EventIInteract
  (bind _manager (Variables|Default|GetManager))
  ;[1 1 1] Interact
  (if (not (Variables|Default|GetbQuestComplete?))
    (if (Variables|/Game/QuestBuilder/Core/QuestData/BP_QuestManager.BP_QuestManager_C|GetbReturn? _manager)
      (if (== (Variables|/Game/QuestBuilder/Core/QuestData/BP_QuestManager.BP_QuestManager_C|GetQuestData _manager) (Variables|Default|GetQuestData))
        (Default|CompleteQuest (Variables|Default|GetManager))
        (Variables|Default|SetbQuestComplete? true))
      (elif (Variables|/Game/QuestBuilder/Core/QuestData/BP_QuestManager.BP_QuestManager_C|GetbQuestActive? (Variables|Default|GetManager))
        (if (== (Variables|/Game/QuestBuilder/Core/QuestData/BP_QuestManager.BP_QuestManager_C|GetQuestData (Variables|Default|GetManager)) (Variables|Default|GetQuestData))
          (CallFunction|OpenTextBox "Thanks for helping, good luck out there!")
          (else
            (CallFunction|OpenTextBox "It looks like you're busy at the moment but please come back to me whenever you're finished.")))
        (else
          (bind _asbp_npc (Utilities|Casting|CastToBP_NPCParent (Components|GetOwner)))
          (Variables|Default|SetbTalking? true)
          (bind _returnvalue (UserInterface|CreateWidget "/Game/QuestBuilder/Core/UI/WBP_StartQuest.WBP_StartQuest_C"))
          (Default|Init _returnvalue (Variables|Default|GetQuestData) (Variables|Default|GetManager) _asbp_npc)
          (UserInterface|Viewport|AddtoViewport _returnvalue 0)
          (Input|SetInputModeUIOnly (Game|GetPlayerController 0) _returnvalue "DoNotLock" false)
          (Pawn|Components|CharacterMovement|SetMovementMode (Variables|/Script/Engine.Character|GetCharacterMovement (Game|GetPlayerCharacter 0)) "MOVE_None" 0))))
    (else
      (CallFunction|OpenTextBox "Thanks! I really appreciate your help. I'll be sure to give you a shout if I need anything!"))))

(fn AddInteractWidget
  (params (Owner :type Actor%20Object%20Reference))
  (bind _returnvalue (Game|AddComponentbyClass Owner "/Script/UMG.WidgetComponent" false (Math|Transform|MakeTransform "0.000000,0.000000,10.000000")))
  (bind _returnvalue_2 (UserInterface|CreateWidget "/Game/QuestBuilder/Core/NPC/WBP_NPC.WBP_NPC_C"))
  (Variables|Default|SetWidget _returnvalue)
  (UserInterface|SetWidget _returnvalue _returnvalue_2)
  (Class|WidgetComponent|SetWidgetSpace _returnvalue "Screen")
  (Rendering|SetVisibility _returnvalue false false))

(fn AddCollider
  (params (Owner :type Actor%20Object%20Reference))
  (bind _returnvalue (Game|AddComponentbyClass Owner "/Script/Engine.SphereComponent" false))
  (bind _output_get (Variables|Default|SetCollider _returnvalue))
  (Components|Sphere|SetSphereRadius _output_get (Variables|Default|GetInteractRadius) true)
  (Collision|BindEventtoOnComponentBeginOverlap (Variables|Default|GetCollider) (EventDispatchers|CreateEvent :!event Custom|BeginOverlap))
  (Collision|BindEventtoOnComponentEndOverlap (Variables|Default|GetCollider) (EventDispatchers|CreateEvent :!event Custom|EndOverlap)))

(fn OpenTextBox
  (params (Text :type String))
  (Variables|Default|SetbTalking? true)
  (bind _returnvalue (UserInterface|CreateWidget "/Game/QuestBuilder/Core/UI/WBP_TextBox.WBP_TextBox_C"))
  (bind _asbp_npc (Utilities|Casting|CastToBP_NPCParent (Components|GetOwner)))
  (Default|Init _returnvalue Text _asbp_npc)
  (UserInterface|Viewport|AddtoViewport _returnvalue 0)
  (Input|SetInputModeUIOnly (Game|GetPlayerController 0) _returnvalue "DoNotLock" false)
  (Pawn|Components|CharacterMovement|SetMovementMode (Variables|/Script/Engine.Character|GetCharacterMovement (Game|GetPlayerCharacter 0)) "MOVE_None" 0))