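; Base NPC actor for the quest builder that turns to face the player while they are within its collider and exposes a text render label.
; BeginPlay initializes the ACNPC component and binds overlap events on its collider.
; Player overlap starts a looping timer that interpolates the actor toward the player on yaw only, and leaving clears it.
; SetText updates the TextRender.
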(event Custom|BeginOverlap
  (params (OverlappedComponent :type Primitive%20Component%20Object%20Reference) (OtherActor :type Actor%20Object%20Reference) (OtherComp :type Primitive%20Component%20Object%20Reference) (OtherBodyIndex :type Integer) (bFromSweep :type Boolean) (SweepResult :type Hit%20Result%20Structure%20%28by%20ref%29))
  ;[1 1 1] BeginOverlap
  (if (== OtherActor (Game|GetPlayerCharacter 0))
    (bind _returnvalue (Utilities|Time|SetTimerbyFunctionName 0 "RotateToPlayer" 0.01 true))
    (Variables|Default|SetRotateTimer _returnvalue)))

(event Custom|EndOverlap
  (params (OverlappedComponent :type Primitive%20Component%20Object%20Reference) (OtherActor :type Actor%20Object%20Reference) (OtherComp :type Primitive%20Component%20Object%20Reference) (OtherBodyIndex :type Integer))
  ;[1 1 1] EndOverlap
  (if (== OtherActor (Game|GetPlayerCharacter 0))
    (Utilities|Time|ClearandInvalidateTimerbyHandle (Variables|Default|GetRotateTimer))))

(event Custom|SetText
  (params (Text :type Text%20%28by%20ref%29))
  (Rendering|Components|TextRender|SetText (Variables|Default|GetTextRender) Text))

(event EventBeginPlay
  (bind _ac_npc (Variables|Default|GetAC_NPC))
  (bind _collider (Variables|/Game/QuestBuilder/Core/NPC/AC_NPC.AC_NPC_C|GetCollider _ac_npc))
  ;[1 1 1] BeginPlay
  (Default|Init _ac_npc)
  (Collision|BindEventtoOnComponentBeginOverlap _collider (EventDispatchers|CreateEvent :!event Custom|BeginOverlap))
  (Collision|BindEventtoOnComponentEndOverlap _collider (EventDispatchers|CreateEvent :!event Custom|EndOverlap)))

(fn ConstructionScript)

(fn RotatetoPlayer
  (Transformation|SetActorRotation (Math|Rotator|MakeRotator 0.0 0.0 (.yaw (Math|Interpolation|RInterpTo (Transformation|GetActorRotation) (Math|Rotator|FindLookatRotation (Transformation|GetActorLocation) (Transformation|GetActorLocation (Game|GetPlayerCharacter 0))) (Utilities|Time|GetWorldDeltaSeconds) 1e+01)))))