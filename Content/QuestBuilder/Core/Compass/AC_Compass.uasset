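; AC_Compass is a component that drives an on-screen compass from the owner's follow camera heading.
; Init stores the owner, then creates and initializes a WBP_Compass widget and adds it to the viewport.
; SetCompass converts the camera's world yaw into a negated, scaled and offset value and passes it to the widget's SetCompassRotation; no tick or timer in this graph calls it.
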(event Custom|Set%20Compass
  ;[1 1 1] Set Compass Rotation
  (Default|SetCompassRotation (Variables|Default|GetCompassRef) (- (* (* (.yaw (Transformation|GetWorldRotation (Variables|/Game/ThirdPerson/Blueprints/BP_ThirdPersonCharacter.BP_ThirdPersonCharacter_C|GetFollowCamera (Variables|Default|GetOwner)))) -1.0) 1e+01) 2.7e+03)))

(event Custom|Init
  (params (Owner :type BP%20Third%20Person%20Character%20Object%20Reference))
  ;[1 1 1] Init
  (Variables|Default|SetOwner Owner)
  (bind _returnvalue (UserInterface|CreateWidget "/Game/QuestBuilder/Core/Compass/WBP_Compass.WBP_Compass_C"))
  (Default|Init _returnvalue (Variables|Default|GetOwner))
  (Variables|Default|SetCompassRef _returnvalue)
  (UserInterface|Viewport|AddtoViewport _returnvalue 0))